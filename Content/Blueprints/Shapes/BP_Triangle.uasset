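; BP_Triangle is a triangle shape actor that tells an overlapping BP_Peasant which shape and color it has entered.
; On begin overlap it calls the parent handler, then writes the triangle's shape index and CurrentShapeColor onto the peasant.
; On end overlap it resets both peasant values to -1, without checking whether they still belong to this triangle.
; Both overlap events also print debug messages.
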(event `self.ReceiveActorBeginOverlap`
  (params (OtherActor :type "Actor Object Reference"))
  (`KismetSystemLibrary.PrintString` "triangle entered")
  (`parent.ReceiveActorBeginOverlap` null)
  (bind _asbp_peasant (cast `/Game/Blueprints/BP_Peasant` OtherActor))
  (set `/Game/Blueprints/BP_Peasant.CurrentEnteredShape` 1 _asbp_peasant)
  (set `/Game/Blueprints/BP_Peasant.CurrentEnteredShapeColor` (`self.CurrentShapeColor`) _asbp_peasant))

(event `self.ReceiveActorEndOverlap`
  (params (OtherActor :type "Actor Object Reference"))
  (`KismetSystemLibrary.PrintString` "triangle exited")
  (bind _asbp_peasant (cast `/Game/Blueprints/BP_Peasant` OtherActor))
  (set `/Game/Blueprints/BP_Peasant.CurrentEnteredShape` -1 _asbp_peasant)
  (set `/Game/Blueprints/BP_Peasant.CurrentEnteredShapeColor` -1 _asbp_peasant))

(fn `UserConstructionScript`
  (`parent.UserConstructionScript`))