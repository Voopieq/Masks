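; Game State Blueprint that runs a level loop in which shapes spawn and are checked against a killzone.
; Each level increments a counter and uses timers and event dispatcher calls to signal level start, shape spawning and killzone checks.
; A killzone check destroys remaining shapes after a delay, while removing the last tracked shape also advances the level.
; Duplicate spawn and killzone events plus unconnected node chains remain in the graph.
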(event `self.ReceiveBeginPlay`
  (`KismetSystemLibrary.Delay` 0.2)
  (`self.StartNewLevel`))

(event `StartNewLevel`
  (`/Engine/EditorBlueprintResources/StandardMacros.IncrementInt` (`self.CurrentLevel`)
    (:`  `
      (`self.StartPreSpawnTimer`)
      (`self.TriggerNewLevel`))))

(event `StartPreSpawnTimer`
  (`KismetSystemLibrary.K2_SetTimerDelegate` (`|CreateDelegate` :!event `Spawn Shape`) 3.0))

(event `Spawn Shape`
  (`self.SpawnShapesEvent`))

(event `StartPreShapeDestroyEvent`
  (`KismetSystemLibrary.K2_SetTimerDelegate` (`|CreateDelegate` :!event `Check Killzone`) 5.0))

(event `Check Killzone`
  (`self.CheckKillzone`)
  ; Clear spawned shapes from map and array
  (`KismetSystemLibrary.Delay` 3.0)
  (for _array_element (`self.SpawnedShapes`)
    (`self.K2_DestroyActor` _array_element))
  (`KismetArrayLibrary.Array_Clear` (`self.SpawnedShapes`))
  (`self.TriggerNewLevel`)
  (`self.StartNewLevel`))

(event `Remove From Spawned Shapes`
  (params (`Spawned Shape` :type "/Game/Blueprints/Shapes/BP_ShapeBase Object Reference"))
  (bind _spawnedshapes (`self.SpawnedShapes`))
  (`self.CheckKillzone`)
  (`KismetArrayLibrary.Array_RemoveItem` _spawnedshapes `Spawned Shape`)
  (if (`KismetArrayLibrary.Array_IsEmpty` _spawnedshapes)
    (`self.StartNewLevel`)))

(event `SpawnShape`
  (`self.SpawnShapesEvent`)
  (`KismetSystemLibrary.K2_SetTimerDelegate` :`Time` 5.0))

(event `CheckKillzone_Event`
  (`self.CheckKillzone`)
  ; Clear spawned shapes from map and array
  (`KismetSystemLibrary.Delay` 3.0)
  (for _array_element (`self.SpawnedShapes`)
    (`self.K2_DestroyActor` _array_element))
  (`KismetArrayLibrary.Array_Clear` (`self.SpawnedShapes`))
  (`/Engine/EditorBlueprintResources/StandardMacros.IncrementInt` (`self.CurrentLevel`)
    (:`  `
      (`self.TriggerNewLevel`))))

(fn `UserConstructionScript`)