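; Player controller that lets the player choose a mask shape and color through an on-screen mask selection widget.
; On BeginPlay it creates the WB_MaskSelection widget, adds it to the viewport and defaults to a red circle mask.
; Enhanced Input actions for four shapes and four colors each call the matching function on the stored widget reference, which handles the selection itself.
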(event `self.ReceiveBeginPlay`
  (bind _maskselectionwidgetref (`self.MaskSelectionWidgetRef`))
  (`self.AddMaskSelectionWidget`)
  (`/Game/Widgets/HUD/WB_MaskSelection.CircleMask` _maskselectionwidgetref)
  (`/Game/Widgets/HUD/WB_MaskSelection.RedColor` _maskselectionwidgetref))

(event `EnhancedInput|/Game/Input/IA_CircleMaskShape`
  (params (ActionValue :type Boolean) (ElapsedSeconds :type "Float (double-precision)") (TriggeredSeconds :type "Float (double-precision)") (InputAction :type "InputAction Object Reference" :default "/Game/Input/IA_CircleMaskShape.IA_CircleMaskShape"))
  ; Iinput to change mask
  (:`Triggered`
    (`/Game/Widgets/HUD/WB_MaskSelection.CircleMask` (`self.MaskSelectionWidgetRef`))))

(event `EnhancedInput|/Game/Input/IA_TriangleMaskShape`
  (params (ActionValue :type Boolean) (ElapsedSeconds :type "Float (double-precision)") (TriggeredSeconds :type "Float (double-precision)") (InputAction :type "InputAction Object Reference" :default "/Game/Input/IA_TriangleMaskShape.IA_TriangleMaskShape"))
  ; Iinput to change mask
  (:`Triggered`
    (`/Game/Widgets/HUD/WB_MaskSelection.TriangleMask` (`self.MaskSelectionWidgetRef`))))

(event `EnhancedInput|/Game/Input/IA_SquareMaskShape`
  (params (ActionValue :type Boolean) (ElapsedSeconds :type "Float (double-precision)") (TriggeredSeconds :type "Float (double-precision)") (InputAction :type "InputAction Object Reference" :default "/Game/Input/IA_SquareMaskShape.IA_SquareMaskShape"))
  ; Iinput to change mask
  (:`Triggered`
    (`/Game/Widgets/HUD/WB_MaskSelection.SquareMask` (`self.MaskSelectionWidgetRef`))))

(event `EnhancedInput|/Game/Input/IA_StarMaskShape`
  (params (ActionValue :type Boolean) (ElapsedSeconds :type "Float (double-precision)") (TriggeredSeconds :type "Float (double-precision)") (InputAction :type "InputAction Object Reference" :default "/Game/Input/IA_StarMaskShape.IA_StarMaskShape"))
  ; Iinput to change mask
  (:`Triggered`
    (`/Game/Widgets/HUD/WB_MaskSelection.StarMask` (`self.MaskSelectionWidgetRef`))))

(event `EnhancedInput|/Game/Input/IA_RedColor`
  (params (ActionValue :type Boolean) (ElapsedSeconds :type "Float (double-precision)") (TriggeredSeconds :type "Float (double-precision)") (InputAction :type "InputAction Object Reference" :default "/Game/Input/IA_RedColor.IA_RedColor"))
  (:`Triggered`
    (`/Game/Widgets/HUD/WB_MaskSelection.RedColor` (`self.MaskSelectionWidgetRef`))))

(event `EnhancedInput|/Game/Input/IA_YellowColor`
  (params (ActionValue :type Boolean) (ElapsedSeconds :type "Float (double-precision)") (TriggeredSeconds :type "Float (double-precision)") (InputAction :type "InputAction Object Reference" :default "/Game/Input/IA_YellowColor.IA_YellowColor"))
  (:`Triggered`
    (`/Game/Widgets/HUD/WB_MaskSelection.YellowColor` (`self.MaskSelectionWidgetRef`))))

(event `EnhancedInput|/Game/Input/IA_GreenColor`
  (params (ActionValue :type Boolean) (ElapsedSeconds :type "Float (double-precision)") (TriggeredSeconds :type "Float (double-precision)") (InputAction :type "InputAction Object Reference" :default "/Game/Input/IA_GreenColor.IA_GreenColor"))
  (:`Triggered`
    (`/Game/Widgets/HUD/WB_MaskSelection.GreenColor` (`self.MaskSelectionWidgetRef`))))

(event `EnhancedInput|/Game/Input/IA_BlueColor`
  (params (ActionValue :type Boolean) (ElapsedSeconds :type "Float (double-precision)") (TriggeredSeconds :type "Float (double-precision)") (InputAction :type "InputAction Object Reference" :default "/Game/Input/IA_BlueColor.IA_BlueColor"))
  (:`Triggered`
    (`/Game/Widgets/HUD/WB_MaskSelection.BlueColor` (`self.MaskSelectionWidgetRef`))))

(fn `AddMaskSelectionWidget`
  (bind _returnvalue (`|CreateWidget` "/Game/Widgets/HUD/WB_MaskSelection.WB_MaskSelection_C"))
  (bind _output_get (set `self.MaskSelectionWidgetRef` _returnvalue))
  (`UserWidget.AddToViewport` _output_get 0))

(fn `UserConstructionScript`)