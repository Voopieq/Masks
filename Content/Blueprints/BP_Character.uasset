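; Player character Blueprint with an orbit-style camera that lets the player click peasants to apply the currently selected mask and color.
; Enhanced Input drives control-rotation-relative movement, clamped spring-arm zoom and pitch-limited camera rotation.
; Rotation works only while its input is active, which hides the otherwise visible cursor and switches input mode.
; Left click traces from the cursor, passing the GameState's mask and color indices to the hit BP_Peasant.
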(event `self.ReceiveBeginPlay`
  (bind _returnvalue (`GameplayStatics.GetPlayerCameraManager` 0))
  (`self.InitInputContext`)
  ; Set camera initial zoom
  (set `SpringArmComponent.TargetArmLength` (`self.CameraMaxZoom`) (`self.SpringArm`))
  ; Set camera max/min view pitch
  (set `PlayerCameraManager.ViewPitchMin` (`self.ViewPitchMin`) _returnvalue)
  (set `PlayerCameraManager.ViewPitchMax` (`self.ViewPitchMax`) _returnvalue)
  (set `PlayerController.bShowMouseCursor` true (`GameplayStatics.GetPlayerController` 0))
  (bind _asbp_game_state (cast `/Game/Blueprints/BP_GameState` (`GameplayStatics.GetGameState`)))
  (set `self.GameStateRef` _asbp_game_state))

(event `EnhancedInput|/Game/Input/IA_Move`
  (params (ActionValue :type "Vector2D Structure") (ElapsedSeconds :type "Float (double-precision)") (TriggeredSeconds :type "Float (double-precision)") (InputAction :type "InputAction Object Reference" :default "/Game/Input/IA_Move.IA_Move"))
  (bind (_returnvalue_roll _returnvalue_pitch _returnvalue_yaw) (`KismetMathLibrary.BreakRotator` (`self.GetControlRotation`)))
  (bind (_returnvalue_roll_2 _returnvalue_pitch_2 _returnvalue_yaw_2) (`KismetMathLibrary.BreakRotator` (`self.GetControlRotation`)))
  ; Movement
  (:`Triggered`
    (`self.AddMovementInput` (`KismetMathLibrary.GetRightVector` (`KismetMathLibrary.MakeRotator` _returnvalue_roll_2 0.0 _returnvalue_yaw_2)) ActionValue_X)
    (`self.AddMovementInput` (`KismetMathLibrary.GetForwardVector` (`KismetMathLibrary.MakeRotator` 0.0 0.0 _returnvalue_yaw)) ActionValue_Y)))

(event `EnhancedInput|/Game/Input/IA_Look`
  (params (ActionValue :type "Vector2D Structure") (ElapsedSeconds :type "Float (double-precision)") (TriggeredSeconds :type "Float (double-precision)") (InputAction :type "InputAction Object Reference" :default "/Game/Input/IA_Look.IA_Look"))
  ; Camera rotation
  (:`Triggered`
    (if (`self.EnableCameraRotation`)
      (`self.AddControllerYawInput` ActionValue_X)
      (`self.AddControllerPitchInput` ActionValue_Y))))

(event `EnhancedInput|/Game/Input/IA_Move`
  (params (ActionValue :type "Vector2D Structure") (ElapsedSeconds :type "Float (double-precision)") (TriggeredSeconds :type "Float (double-precision)") (InputAction :type "InputAction Object Reference" :default "/Game/Input/IA_Move.IA_Move"))
  ; NOTE: Allows to rotate camera with A and D
)

(event `EnhancedInput|/Game/Input/IA_MouseWheel`
  (params (ActionValue :type "Float (double-precision)") (ElapsedSeconds :type "Float (double-precision)") (TriggeredSeconds :type "Float (double-precision)") (InputAction :type "InputAction Object Reference" :default "/Game/Input/IA_MouseWheel.IA_MouseWheel"))
  (bind _springarm (`self.SpringArm`))
  ; Camera Zoom In/Out
  (:`Triggered`
    (set `SpringArmComponent.TargetArmLength` (`KismetMathLibrary.FClamp` (+ (* ActionValue (`self.CameraZoomSpeed`)) (`SpringArmComponent.TargetArmLength` _springarm)) (`self.CameraMinZoom`) (`self.CameraMaxZoom`)) _springarm)))

(event `EnhancedInput|/Game/Input/IA_EnableCameraRotate`
  (params (ActionValue :type Boolean) (ElapsedSeconds :type "Float (double-precision)") (TriggeredSeconds :type "Float (double-precision)") (InputAction :type "InputAction Object Reference" :default "/Game/Input/IA_EnableCameraRotate.IA_EnableCameraRotate"))
  (bind _returnvalue (`GameplayStatics.GetPlayerController` 0))
  ; Enable/disable camera rotation, show/hide mouse cursor
  (:`Triggered`
    (set `self.EnableCameraRotation` ActionValue)
    (`WidgetBlueprintLibrary.SetInputMode_GameOnly` _returnvalue)
    (set `PlayerController.bShowMouseCursor` false _returnvalue))
  (:`Completed`
    (set `self.EnableCameraRotation` false)
    (`WidgetBlueprintLibrary.SetInputMode_GameAndUIEx` _returnvalue null)
    (set `PlayerController.bShowMouseCursor` true _returnvalue)))

(event `Key|LeftMouseButton`
  (params (Key :type "Key Structure"))
  (bind _gamestateref (`self.GameStateRef`))
  (bind (_worldlocation _worlddirection) (`PlayerController.DeprojectMousePositionToWorld` (`GameplayStatics.GetPlayerController` 0)))
  (:`Pressed`
    (bind _outhit (`KismetSystemLibrary.LineTraceSingle` :`Start` _worldlocation :`End` (+ _worldlocation (* _worlddirection 5000.0)) :`TraceChannel` "TraceTypeQuery1" :`DrawDebugType` "ForDuration"))
    (bind _asbp_peasant (cast `/Game/Blueprints/BP_Peasant` (`.HitActor` (`GameplayStatics.BreakHitResult` _outhit))))
    (`/Game/Blueprints/BP_Peasant.ChangeMask` _asbp_peasant (`/Game/Blueprints/BP_GameState.CurrentMaskIndex` _gamestateref))
    (`/Game/Blueprints/BP_Peasant.ChangeColor` _asbp_peasant (`/Game/Blueprints/BP_GameState.CurrentColorIndex` _gamestateref))))

(fn `InitInputContext`
  (bind _asbp_player_controller (cast `/Game/Blueprints/BP_PlayerController` (`self.GetController`)))
  (`EnhancedInputSubsystemInterface.AddMappingContext` (pcsubsystem `EnhancedInputLocalPlayerSubsystem` _asbp_player_controller) "/Game/Input/IMC_Character.IMC_Character" 0 (struct)))

(fn `UserConstructionScript`)