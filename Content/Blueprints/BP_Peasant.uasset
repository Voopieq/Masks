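; BP_Peasant is a wandering NPC whose mask shape and color decide whether it survives killzone checks.
; It loops AIMoveTo to random nearby reachable points after each success, while its head turns toward the player camera every tick.
; ChangeMask and ChangeColor set the visible mask and material.
; On the GameState's killzone event, a peasant inside a shape with mismatched shape or color decrements the peasant count and is destroyed.
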(event `self.ReceiveTick`
  (params (DeltaSeconds :type "Float (single-precision)"))
  (bind _head (`self.head`))
  (`SceneComponent.K2_SetWorldRotation` _head (`KismetMathLibrary.FindLookAtRotation` (`SceneComponent.K2_GetComponentLocation` _head) (`PlayerCameraManager.GetCameraLocation` (`GameplayStatics.GetPlayerCameraManager` 0))) false false))

(event `self.ReceiveBeginPlay`
  (`self.NPCMove`)
  (bind _asbp_game_state (cast `/Game/Blueprints/BP_GameState` (`GameplayStatics.GetGameState`)))
  (bind _output_get (set `self.As BP Game State` _asbp_game_state))
  ; Check killzone event
  (add `/Game/Blueprints/BP_GameState.CheckKillzone` _output_get (delegate `Check Killzone`)))

(event `Check Killzone`
  ; Check killzone event
  (if (< (`self.CurrentEnteredShape`) 0)
    _
    (elif (== (`self.CurrentEnteredShape`) (`self.CurrentMaskIndex`))
      ;; Current mask shape is same as entered shape. Check mask color
      (if (not (== (`self.CurrentColorIndex`) (`self.CurrentEnteredShapeColor`)))
        (`/Game/Blueprints/BP_GameState.Decrement Peasant` (`self.As BP Game State`))
        (`self.K2_DestroyActor`))
      (else
        ;; Current mask is not the same as entered shape
        (`/Game/Blueprints/BP_GameState.Decrement Peasant` (`self.As BP Game State`))
        (`self.K2_DestroyActor`)))))

(event `NPCMove`
  (`|AIMoveTo` self (`NavigationSystemV1.K2_GetRandomReachablePointInRadius` (`self.K2_GetActorLocation`) 500.0 null null) null
    (:`OnSuccess`
      (`KismetSystemLibrary.Delay` 0.5)
      (`self.NPCMove`))))

(event `ChangeMask`
  (params (type :type Integer))
  (bind _round_mask (`self.round_mask`))
  (bind _triangle_mask (`self.triangle_mask`))
  (bind _square_mask (`self.square_mask`))
  (bind _star_mask (`self.star_mask`))
  ; Change mask
  (`SceneComponent.SetVisibility` (`self.round_mask`) false false)
  (`SceneComponent.SetVisibility` (`self.triangle_mask`) false false)
  (`SceneComponent.SetVisibility` (`self.square_mask`) false false)
  (`SceneComponent.SetVisibility` (`self.star_mask`) false false)
  (switch `int` type
    (:`0`
      (`SceneComponent.SetVisibility` _round_mask true false)
      (set `self.CurrentMask` _round_mask)
      (set `self.CurrentMaskIndex` 0))
    (:`1`
      (`SceneComponent.SetVisibility` _triangle_mask true false)
      (set `self.CurrentMask` _triangle_mask)
      (set `self.CurrentMaskIndex` 1))
    (:`2`
      (`SceneComponent.SetVisibility` _square_mask true false)
      (set `self.CurrentMask` _square_mask)
      (set `self.CurrentMaskIndex` 2))
    (:`3`
      (`SceneComponent.SetVisibility` _star_mask true false)
      (set `self.CurrentMask` _star_mask)
      (set `self.CurrentMaskIndex` 3))))

(event `ChangeColor`
  (params (type :type Integer))
  ; Change mask color
  (switch `int` type
    (:`0`
      (`PrimitiveComponent.SetMaterial` (`self.CurrentMask`) 0 "/Game/Assets/m_red.m_red")
      (set `self.CurrentColorIndex` 0))
    (:`1`
      (`PrimitiveComponent.SetMaterial` (`self.CurrentMask`) 0 "/Game/Assets/m_green.m_green")
      (set `self.CurrentColorIndex` 1))
    (:`2`
      (`PrimitiveComponent.SetMaterial` (`self.CurrentMask`) 0 "/Game/Assets/m_blue.m_blue")
      (set `self.CurrentColorIndex` 2))
    (:`3`
      (`PrimitiveComponent.SetMaterial` (`self.CurrentMask`) 0 "/Game/Assets/m_yellow.m_yellow")
      (set `self.CurrentColorIndex` 3))))

(fn `UserConstructionScript`)